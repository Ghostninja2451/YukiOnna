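; ObjectiveBP is a collectable objective actor that the player picks up with the Interaction input.
; A box overlap with PlayerSurvive enables input on the actor, and leaving the box disables it.
; On interaction it decrements CollectableLeft on MyGamemode, adds a Collectable widget to the viewport, and destroys itself.
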(event `InputAction|Interaction`
  (params (Key :type "Key Structure"))
  (:`Pressed`
    (bind _asmy_gamemode (cast `/Game/MyPlayer/MyGamemode` (`GameplayStatics.GetGameMode`)))
    (bind _result (`/Engine/EditorBlueprintResources/StandardMacros.DecrementInt` (`/Game/MyPlayer/MyGamemode.Collectable Left` _asmy_gamemode))
      (:`  `
        (set `/Game/MyPlayer/MyGamemode.Collectable Left` _result _asmy_gamemode)
        (bind _returnvalue (`|CreateWidget` "/Game/DisplayCanvas/Collectable.Collectable_C"))
        (`UserWidget.AddToViewport` _returnvalue 0)
        (`self.K2_DestroyActor`)))))

(event `self.Box.OnComponentBeginOverlap`
  (params (OverlappedComponent :type "PrimitiveComponent Object Reference") (OtherActor :type "Actor Object Reference") (OtherComp :type "PrimitiveComponent Object Reference") (OtherBodyIndex :type Integer) (bFromSweep :type Boolean) (SweepResult :type "HitResult Structure (by ref)"))
  (cast `/Game/MyPlayer/PlayerSurvive` OtherActor)
  (`self.EnableInput` (`GameplayStatics.GetPlayerController` 0)))

(event `self.Box.OnComponentEndOverlap`
  (params (OverlappedComponent :type "PrimitiveComponent Object Reference") (OtherActor :type "Actor Object Reference") (OtherComp :type "PrimitiveComponent Object Reference") (OtherBodyIndex :type Integer))
  (cast `/Game/MyPlayer/PlayerSurvive` OtherActor)
  (`self.DisableInput` (`GameplayStatics.GetPlayerController` 0)))

(fn `UserConstructionScript`)